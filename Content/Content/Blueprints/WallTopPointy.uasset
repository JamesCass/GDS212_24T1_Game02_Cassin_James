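; WallTopPointy is a destructible wooden wall-top piece that cracks, then breaks, under fast impacts.
; A boulder overlapping WoodCollider passes its speed to DealDamage, while any hit on WoodCube passes the cube's own speed.
; Each impact above the velocity threshold advances a damage state: the first swaps wall and roof materials to cracked versions, the second destroys the actor.
; Particle emitter spawns are present but unconnected.
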(event `self.WoodCollider.OnComponentBeginOverlap`
  (params (OverlappedComponent :type "PrimitiveComponent Object Reference") (OtherActor :type "Actor Object Reference") (OtherComp :type "PrimitiveComponent Object Reference") (OtherBodyIndex :type Integer) (bFromSweep :type Boolean) (SweepResult :type "HitResult Structure (by ref)"))
  (bind _asboulder_bp (cast `/Game/Content/Blueprints/Boulder_BP` OtherActor))
  (`self.DealDamage` (`KismetMathLibrary.VSize` (`SceneComponent.GetComponentVelocity` (`/Game/Content/Blueprints/Boulder_BP.Boulder` _asboulder_bp))) 500.0))

(event `self.WoodCube.OnComponentHit`
  (params (HitComponent :type "PrimitiveComponent Object Reference") (OtherActor :type "Actor Object Reference") (OtherComp :type "PrimitiveComponent Object Reference") (NormalImpulse :type "Vector Structure") (Hit :type "HitResult Structure (by ref)"))
  (`self.DealDamage` (`KismetMathLibrary.VSize` (`SceneComponent.GetComponentVelocity` (`self.WoodCube`))) 500.0))

(fn `DealDamage`
  (params (Velocity :type "Float (double-precision)") (VelocityThreshold :type "Float (double-precision)"))
  (locals (IntSwitch :type Integer :default 0))
  (bind _woodcube (`self.WoodCube`))
  (if (> Velocity VelocityThreshold)
    (bind _result (`/Engine/EditorBlueprintResources/StandardMacros.IncrementInt` (`self.IntDestroyedState`))
      (:`  `
        (switch `int` _result
          (:`1`
            (`PrimitiveComponent.SetMaterial` _woodcube 0 "/Game/Content/Assets/KenneyCastle/WallCracked.WallCracked")
            (`PrimitiveComponent.SetMaterial` _woodcube 1 "/Game/Content/Assets/KenneyCastle/wallDarkCracked.wallDarkCracked")
            (`PrimitiveComponent.SetMaterial` _woodcube 2 "/Game/Content/Assets/KenneyCastle/RoofCracked.RoofCracked"))
          (:`2`
            (`self.K2_DestroyActor`)))))))

(fn `UserConstructionScript`)