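; WallBottom_BP is a destructible wall base piece that cracks and then breaks under fast impacts.
; A Boulder_BP overlapping the collider passes the boulder's speed to DealDamage, while any hit on the base mesh passes the mesh's own speed.
; Above the speed threshold, a damage counter advances, first swapping in cracked materials, then destroying the actor.
; Two emitter spawns are unconnected and never run.
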(event `self.WallBaseCollider.OnComponentBeginOverlap`
  (params (OverlappedComponent :type "PrimitiveComponent Object Reference") (OtherActor :type "Actor Object Reference") (OtherComp :type "PrimitiveComponent Object Reference") (OtherBodyIndex :type Integer) (bFromSweep :type Boolean) (SweepResult :type "HitResult Structure (by ref)"))
  (bind _asboulder_bp (cast `/Game/Content/Blueprints/Boulder_BP` OtherActor))
  (`self.DealDamage` (`KismetMathLibrary.VSize` (`SceneComponent.GetComponentVelocity` (`/Game/Content/Blueprints/Boulder_BP.Boulder` _asboulder_bp))) 500.0))

(event `self.towerSquareBase_towerSquareBase.OnComponentHit`
  (params (HitComponent :type "PrimitiveComponent Object Reference") (OtherActor :type "Actor Object Reference") (OtherComp :type "PrimitiveComponent Object Reference") (NormalImpulse :type "Vector Structure") (Hit :type "HitResult Structure (by ref)"))
  (`self.DealDamage` (`KismetMathLibrary.VSize` (`SceneComponent.GetComponentVelocity` (`self.towerSquareBase_towerSquareBase`))) 500.0))

(fn `DealDamage`
  (params (Velocity :type "Float (double-precision)") (`Velocity Threshold` :type "Float (double-precision)"))
  (bind _towersquarebase_towersquarebase (`self.towerSquareBase_towerSquareBase`))
  (if (> Velocity `Velocity Threshold`)
    (bind _result (`/Engine/EditorBlueprintResources/StandardMacros.IncrementInt` (`self.IntDestroyedState`))
      (:`  `
        (switch `int` _result
          (:`1`
            (`PrimitiveComponent.SetMaterial` _towersquarebase_towersquarebase 0 "/Game/Content/Assets/KenneyCastle/WallCracked.WallCracked")
            (`PrimitiveComponent.SetMaterial` _towersquarebase_towersquarebase 1 "/Game/Content/Assets/KenneyCastle/wallDarkCracked.wallDarkCracked"))
          (:`2`
            (`self.K2_DestroyActor`)))))))

(fn `UserConstructionScript`)