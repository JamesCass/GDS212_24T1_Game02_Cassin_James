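; Trebuchet player weapon that launches boulders at knights by touch drag, with limited ammo shown on a text render.
; While touched, Tick turns drag offset into launch velocity and spawns prediction objects along the simulated path.
; Release fires a boulder with that velocity, then after a delay shows level-complete UI if no knights remain.
; Releasing with no ammo shows the loss UI; both end screens pause the game.
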(event `self.ReceiveBeginPlay`
  ;[1 1 1] ammo
  (`|ExecutionSequence`
    (:`then_0`
      (`KismetSystemLibrary.Delay` 0.1)
      (`TextRenderComponent.K2_SetText` (`self.TextRender`) (`KismetTextLibrary.Conv_IntToText` (`self.RemainingAmmo`))))
    (:`then_1`
      (bind _returnvalue (`|CreateWidget` "/Game/Content/UI/Game_UI.Game_UI_C"))
      (`UserWidget.AddToViewport` _returnvalue 0))))

(event `self.ReceiveTick`
  (params (DeltaSeconds :type "Float (single-precision)"))
  ;[1 1 1] Projectile prediction line
  (if (`self.ShouldPredict`)
    (bind _returnvalue (`WidgetLayoutLibrary.GetMousePositionOnViewport`))
    (bind (_returnvalue_x _returnvalue_y) (`KismetMathLibrary.BreakVector2D` (- _returnvalue (`self.ClickOriginalPosition`))))
    (bind (_outhit _outpathpositions) (`GameplayStatics.Blueprint_PredictProjectilePath_ByTraceChannel` :`StartPos` (`SceneComponent.K2_GetComponentLocation` (`self.Launch Position`)) :`LaunchVelocity` (`KismetMathLibrary.MakeVector` 0.0 (* _returnvalue_x 6.0) _returnvalue_y) :`ProjectileRadius` 2.0 :`DrawDebugTime` 1.0 :`SimFrequency` 10.0 :`MaxSimTime` 1.0))
    (for _array_element _outpathpositions
      (`|SpawnActorFromClass` "/Game/Content/Blueprints/PredictionObject_BP.PredictionObject_BP_C" (`KismetMathLibrary.MakeTransform` _array_element) "Undefined" "MultiplyWithRoot" null null))))

(event `InputTouch`
  (params (Location :type "Vector Structure") (FingerIndex :type "ETouchIndex Enum"))
  (:`Pressed`
    (set `self.ShouldPredict` true)
    (bind _returnvalue (`WidgetLayoutLibrary.GetMousePositionOnViewport`))
    (set `self.ClickOriginalPosition` _returnvalue))
  (:`Released`
    (if (< 0 (`self.RemainingAmmo`))
      (set `self.ShouldPredict` false)
      (bind _returnvalue_2 (`|SpawnActorFromClass` "/Game/Content/Blueprints/Boulder_BP.Boulder_BP_C" (`KismetMathLibrary.MakeTransform` (`SceneComponent.K2_GetComponentLocation` (`self.Launch Position`))) "Undefined" "MultiplyWithRoot" null null))
      (bind (_returnvalue_x _returnvalue_y) (`KismetMathLibrary.BreakVector2D` (- (stale `self.ReceiveTick` _returnvalue) (`self.ClickOriginalPosition`))))
      (`PrimitiveComponent.AddImpulse` (`/Game/Content/Blueprints/Boulder_BP.Boulder` _returnvalue_2) (`KismetMathLibrary.MakeVector` 0.0 (* _returnvalue_x 6.0) _returnvalue_y) "None" true)
      (bind _result (`/Engine/EditorBlueprintResources/StandardMacros.DecrementInt` (`self.RemainingAmmo`))
        (:`  `
          (`TextRenderComponent.K2_SetText` (`self.TextRender`) (`KismetTextLibrary.Conv_IntToText` _result))
          (`KismetSystemLibrary.Delay` 6.0)
          (bind _outactors (`GameplayStatics.GetAllActorsOfClass` "/Game/Content/Blueprints/Knight-BP.Knight-BP_C"))
          (if (== (`KismetArrayLibrary.Array_Length` _outactors) 0)
            (bind _returnvalue_3 (`|CreateWidget` "/Game/Content/UI/LevelComplete_UI.LevelComplete_UI_C"))
            (`UserWidget.AddToViewport` _returnvalue_3 0)
            (`GameplayStatics.SetGamePaused` true))))
      (else
        (set `self.ShouldPredict` false)
        (`KismetSystemLibrary.Delay` 2.0)
        (bind _returnvalue_4 (`|CreateWidget` "/Game/Content/UI/Loss_UI.Loss_UI_C"))
        (`UserWidget.AddToViewport` _returnvalue_4 0)
        (`GameplayStatics.SetGamePaused` true)))))

(fn `UserConstructionScript`)